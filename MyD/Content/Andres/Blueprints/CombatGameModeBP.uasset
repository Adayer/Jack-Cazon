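; CombatGameModeBP is a combat game mode Blueprint that sets up the player's action UI and holds a debug-style kill event.
; InitializeActionsWidget creates an ActionsMenuWidget for player 0 and adds it to the viewport.
; KillRandom, despite its name, deals 1000 damage to the character after the current turn index in TurnOrderDataList, wrapping around the list.
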(event Custom|KillRandom
  (bind _turnorderdatalist (Variables|Default|GetturnOrderDataList))
  (bind _returnvalue (Class|CombatGameMode|GetTurnIndex))
  (Class|CharacterActor|RecieveDamage (Class|TurnOrderData|GetCharacterBP (Utilities|Array|Get(acopy) _turnorderdatalist (Math|Integer|%(Integer) (+ _returnvalue 1) (Utilities|Array|Length _turnorderdatalist)))) 1000))

(event EventInitializeActionsWidget
  (bind _returnvalue (UserInterface|CreateWidget "/Game/Marcos/ActionsMenuWidget.ActionsMenuWidget_C" (Game|GetPlayerController 0)))
  (UserInterface|Viewport|AddtoViewport _returnvalue 0))

(fn ConstructionScript)