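; Test character for turn-based combat that takes player control when its turn starts.
; StartTurn has player controller 0 possess it.
; M teleports it to a random entry in Targets, rerolling until it differs from the current Index, so a single-entry array can loop forever.
; N calls ContinueCombat on CombatGameModeBP; both keys use DoOnce gates that reset on release.
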(event EventStartTurn
  (Pawn|Possess (Game|GetPlayerController 0) self))

(event Input|KeyboardEvents|M
  (params (Key :type Key%20Structure :default "None"))
  (:Pressed
    (Utilities|FlowControl|DoOnce false :!label _label
      (:Completed
        (Variables|Default|SetRandValue (Math|Random|RandomIntegerinRange 0 (- (Utilities|Array|Length (Variables|Default|GetTargets)) 1)))
        (while (== (Variables|Default|GetRandValue) (Variables|Default|GetIndex))
          (Variables|Default|SetRandValue (Math|Random|RandomIntegerinRange 0 (- (Utilities|Array|Length (Variables|Default|GetTargets)) 1))))
        (bind _output_get (Variables|Default|SetIndex (Variables|Default|GetRandValue)))
        (Transformation|SetActorLocation (Transformation|GetActorLocation (Utilities|Array|Get(acopy) (Variables|Default|GetTargets) _output_get)) false false))))
  (:Released
    (goto _label Reset)))

(event Input|KeyboardEvents|N
  (params (Key :type Key%20Structure :default "None"))
  (:Pressed
    (Utilities|FlowControl|DoOnce false :!label _label
      (:Completed
        (bind _ascombat_game_mode_bp (Utilities|Casting|CastToCombatGameModeBP (Game|GetGameMode)))
        (Class|CombatGameMode|ContinueCombat _ascombat_game_mode_bp))))
  (:Released
    (goto _label Reset)))

(fn ConstructionScript)